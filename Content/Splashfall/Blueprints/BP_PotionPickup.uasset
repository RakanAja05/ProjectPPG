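; BP_PotionPickup is a respawning pickup that grants BP_Player one potion on overlap.
; It only triggers while available and when the player is below MaxPotionCount.
; Once collected it hides, disables collision, then restores itself after a RespawnTime delay instead of being destroyed.
; The construction script builds the look from a scaled cylinder mesh attached to the overlap-only collision component, with mesh collision disabled.
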(event `self.ReceiveActorBeginOverlap`
  (params (OtherActor :type "Actor Object Reference"))
  (if (`self.bIsAvailable`)
    (bind _asbp_player (cast `/Game/Characters/BP_Player` OtherActor))
    (bind _potioncount (`/Game/Characters/BP_Player.PotionCount` _asbp_player))
    (if (< _potioncount (`/Game/Characters/BP_Player.MaxPotionCount` _asbp_player))
      (set `/Game/Characters/BP_Player.PotionCount` (+ _potioncount 1) _asbp_player)
      (set `self.bIsAvailable` false)
      (`self.SetActorHiddenInGame` true)
      (`self.SetActorEnableCollision` false)
      (`KismetSystemLibrary.Delay` (`self.RespawnTime`))
      (`self.SetActorHiddenInGame` false)
      (`self.SetActorEnableCollision` true)
      (set `self.bIsAvailable` true))))

(fn `UserConstructionScript`
  (bind _pickupcollision (`self.PickupCollision`))
  (bind _pickupmesh (`self.PickupMesh`))
  (`StaticMeshComponent.SetStaticMesh` _pickupmesh "/Engine/BasicShapes/Cylinder.Cylinder")
  (`PrimitiveComponent.SetMaterial` _pickupmesh 0 "/Game/Splashfall/Materials/MI_PotionPickup.MI_PotionPickup")
  (`SceneComponent.K2_AttachToComponent` _pickupmesh _pickupcollision "None" "KeepRelative" "KeepRelative" "KeepRelative" true)
  (`SceneComponent.K2_SetRelativeLocation` _pickupmesh (`KismetMathLibrary.MakeVector` 0.0 0.0 20.0) false false)
  (`SceneComponent.SetRelativeScale3D` _pickupmesh (`KismetMathLibrary.MakeVector` 0.4 0.4 0.4))
  (`PrimitiveComponent.SetCollisionProfileName` _pickupcollision "OverlapAllDynamic" true)
  (`PrimitiveComponent.SetCollisionProfileName` _pickupmesh "NoCollision" true))