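; Poison area-of-effect actor for Splashfall that shows a player-colored zone on a flattened mesh.
; The construction script configures an overlap sphere with the non-colliding visual mesh attached and scaled to match it.
; On BeginPlay it casts its owner to BP_Player and picks the P1 or P2 poison material from PlayerIndex.
; This graph contains no active overlap or damage logic.
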(event `self.ReceiveBeginPlay`
  (bind _aoemesh (`self.AOEMesh`))
  (bind _asbp_player (cast `/Game/Characters/BP_Player` (`self.GetOwner`)))
  (if (== (`/Game/Characters/BP_Player.PlayerIndex` _asbp_player) 0)
    (`PrimitiveComponent.SetMaterial` _aoemesh 0 "/Game/Splashfall/Materials/MI_Poison_P1.MI_Poison_P1")
    (else
      (`PrimitiveComponent.SetMaterial` _aoemesh 0 "/Game/Splashfall/Materials/MI_Poison_P2.MI_Poison_P2"))))

(fn `UserConstructionScript`
  (bind _aoecollision (`self.AOECollision`))
  (bind _aoemesh (`self.AOEMesh`))
  (`SceneComponent.K2_AttachToComponent` _aoecollision (`self.DefaultSceneRoot`) "None" "KeepRelative" "KeepRelative" "KeepRelative" true)
  (`SceneComponent.K2_SetRelativeLocation` _aoecollision (`KismetMathLibrary.MakeVector` 0.0) false false)
  (`SphereComponent.SetSphereRadius` _aoecollision 275.0 true)
  (`PrimitiveComponent.SetCollisionProfileName` _aoecollision "OverlapAllDynamic" true)
  (set `PrimitiveComponent.bGenerateOverlapEvents` true _aoecollision)
  (`SceneComponent.K2_AttachToComponent` _aoemesh _aoecollision "None" "KeepRelative" "KeepRelative" "KeepRelative" true)
  (`SceneComponent.K2_SetRelativeLocation` _aoemesh (`KismetMathLibrary.MakeVector` 0.0 0.0 10.0) false false)
  (`SceneComponent.SetRelativeScale3D` _aoemesh (`KismetMathLibrary.MakeVector` 5.5 5.5 0.2))
  (`PrimitiveComponent.SetCollisionProfileName` _aoemesh "NoCollision" true))