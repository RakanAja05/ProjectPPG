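; Poison projectile that bursts into a BP_PoisonAOE area effect where it hits anything other than its owner, then destroys itself.
; The construction script makes the collision sphere the blocking, hit-notifying body that projectile movement drives, with the mesh as non-colliding visual.
; BeginPlay makes the sphere ignore the owner while moving, and InitThrowVelocity sets the launch velocity.
; Several unconnected debug copies of the hit logic remain in the event graph.
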(event `self.ReceiveBeginPlay`
  (bind _collisionsphere (`self.CollisionSphere`))
  (`MovementComponent.SetUpdatedComponent` (`self.ProjectileMovement`) _collisionsphere)
  (`PrimitiveComponent.IgnoreActorWhenMoving` _collisionsphere (`self.GetOwner`) true))

(event `self.ReceiveHit`
  (params (MyComp :type "PrimitiveComponent Object Reference") (Other :type "Actor Object Reference") (OtherComp :type "PrimitiveComponent Object Reference") (bSelfMoved :type Boolean) (HitLocation :type "Vector Structure") (HitNormal :type "Vector Structure") (NormalImpulse :type "Vector Structure") (Hit :type "HitResult Structure (by ref)"))
  (if (!= Other (`self.GetOwner`))
    (`|SpawnActorFromClass` "/Game/Splashfall/Blueprints/BP_PoisonAOE.BP_PoisonAOE_C" (`KismetMathLibrary.MakeTransform` HitLocation (`KismetMathLibrary.MakeRotator` 0.0) (`KismetMathLibrary.MakeVector` 1.0 1.0 1.0)) "AlwaysSpawn" "MultiplyWithRoot" (`self.GetOwner`) null)
    (`self.K2_DestroyActor` self)))

(fn `InitThrowVelocity`
  (params (NewVelocity :type "Vector Structure"))
  (set `MovementComponent.Velocity` NewVelocity (`self.ProjectileMovement`)))

(fn `UserConstructionScript`
  (bind _collisionsphere (`self.CollisionSphere`))
  (bind _projectilemesh (`self.ProjectileMesh`))
  (`SceneComponent.K2_AttachToComponent` _projectilemesh _collisionsphere "None" "KeepRelative" "KeepRelative" "KeepRelative" true)
  (`MovementComponent.SetUpdatedComponent` (`self.ProjectileMovement`) _collisionsphere)
  (`PrimitiveComponent.SetCollisionProfileName` _collisionsphere "BlockAllDynamic" true)
  (`PrimitiveComponent.SetNotifyRigidBodyCollision` _collisionsphere true)
  (`PrimitiveComponent.SetCollisionProfileName` _projectilemesh "NoCollision" true))